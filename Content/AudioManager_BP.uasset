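; Audio manager Blueprint that grows the Ball1 component in response to captured audio.
; It starts its AudioCapture component and resets Ball1 to unit scale on BeginPlay.
; Each envelope-follower value is printed and added to a running size, which sets Ball1's uniform scale.
; The size accumulates with no clamp or decay, so the ball does not track the current level.
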(event `self.ReceiveBeginPlay`
  (`SynthComponent.Start` (`self.AudioCapture`))
  (set `self.ball1Size` 1.0)
  (`SceneComponent.SetRelativeScale3D` (`self.ball1`) (1.0 1.0 1.0)))

(event `self.AudioCapture.OnAudioEnvelopeValue`
  (params (EnvelopeValue :type "Float (single-precision)"))
  (`KismetSystemLibrary.PrintString` (`KismetStringLibrary.Conv_DoubleToString` EnvelopeValue))
  (bind _output_get (set `self.ball1Size` (+ (stale _output_get) EnvelopeValue)))
  (`SceneComponent.SetRelativeScale3D` (`self.ball1`) (`KismetMathLibrary.Conv_DoubleToVector` _output_get)))

(fn `UserConstructionScript`)