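; Game actor for a four-player microphone blowing game, where each player inflates their own ball during a timed turn.
; BeginPlay starts audio capture and runs the turns as a fixed chain of delays and sound cues that sets ActivePlayer.
; The capture's envelope event scales the active player's ball through GrowthByVolumeMacro, whose formula slows growth as the ball gets bigger.
; Escape quits the game.
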(event `self.ReceiveBeginPlay`
  (bind _blowtime (`self.BlowTime`))
  (bind _returnvalue (`KismetMathLibrary.Conv_DoubleToVector` (`self.ball1Size`)))
  (`SynthComponent.Start` (`self.AudioCapture`))
  (`SceneComponent.SetRelativeScale3D` (`self.ball1`) _returnvalue)
  (`SceneComponent.SetRelativeScale3D` (`self.ball2`) _returnvalue)
  (`SceneComponent.SetRelativeScale3D` (`self.ball3`) (0.0 0.0 0.0))
  (`SceneComponent.SetRelativeScale3D` (`self.ball4`) (0.0 0.0 0.0))
  ; Gameloop
  (`KismetSystemLibrary.Delay` 0.5)
  (`AddComponent|NODE_AddAudioComponent-0`)
  (`KismetSystemLibrary.Delay` 1.8)
  (set `self.ActivePlayer` 1)
  (`KismetSystemLibrary.Delay` _blowtime)
  (`AddComponent|NODE_AddAudioComponent-1`)
  (set `self.ActivePlayer` 0)
  (`KismetSystemLibrary.Delay` 0.5)
  (`AddComponent|NODE_AddAudioComponent-5`)
  (`KismetSystemLibrary.Delay` 2.3)
  (set `self.ActivePlayer` 2)
  (`KismetSystemLibrary.Delay` _blowtime)
  (`AddComponent|NODE_AddAudioComponent-3`)
  (set `self.ActivePlayer` 0)
  (`KismetSystemLibrary.Delay` 0.5)
  (`AddComponent|NODE_AddAudioComponent-6`)
  (`KismetSystemLibrary.Delay` 2.2)
  (set `self.ActivePlayer` 3)
  (`KismetSystemLibrary.Delay` _blowtime)
  (`AddComponent|NODE_AddAudioComponent-2`)
  (set `self.ActivePlayer` 0)
  (`KismetSystemLibrary.Delay` 0.5)
  (`AddComponent|NODE_AddAudioComponent-7`)
  (`KismetSystemLibrary.Delay` 2.2)
  (set `self.ActivePlayer` 4)
  (`KismetSystemLibrary.Delay` _blowtime)
  (`AddComponent|NODE_AddAudioComponent-4`)
  (set `self.ActivePlayer` 0))

(event `self.AudioCapture.OnAudioEnvelopeValue`
  (params (EnvelopeValue :type "Float (single-precision)"))
  ; listening -> growing
  (switch `int` (`self.ActivePlayer`)
    (:`1`
      (bind (_newballsize _sizeasvector) (`self.GrowthByVolume_Macro` (stale _output_get) EnvelopeValue))
      ;; if player 1 -> set ball1 size
      (bind _output_get (set `self.ball1Size` _newballsize))
      (`SceneComponent.SetRelativeScale3D` (`self.ball1`) _sizeasvector))
    (:`2`
      (bind (_newballsize_2 _sizeasvector_2) (`self.GrowthByVolume_Macro` (stale _output_get_2) EnvelopeValue))
      ;; 2
      (bind _output_get_2 (set `self.ball2Size` _newballsize_2))
      (`SceneComponent.SetRelativeScale3D` (`self.ball2`) _sizeasvector_2))
    (:`3`
      (bind (_newballsize_3 _sizeasvector_3) (`self.GrowthByVolume_Macro` (stale _output_get_3) EnvelopeValue))
      ;; 3
      (bind _output_get_3 (set `self.ball3Size` _newballsize_3))
      (`SceneComponent.SetRelativeScale3D` (`self.ball3`) _sizeasvector_3))
    (:`4`
      (bind (_newballsize_4 _sizeasvector_4) (`self.GrowthByVolume_Macro` (stale _output_get_4) EnvelopeValue))
      ;; 4
      (bind _output_get_4 (set `self.ball4Size` _newballsize_4))
      (`SceneComponent.SetRelativeScale3D` (`self.ball4`) _sizeasvector_4))))

(event `Key|Escape`
  (params (Key :type "Key Structure"))
  (:`Pressed`
    (`KismetSystemLibrary.QuitGame` null "Quit")))

(fn `GrowBySoundFunction`
  (params (InputPin :type "Float (single-precision)"))
  (`KismetSystemLibrary.PrintString` (`KismetStringLibrary.Conv_DoubleToString` InputPin))
  (bind _output_get (set `self.ball1Size` (+ (stale _output_get) InputPin)))
  (`SceneComponent.SetRelativeScale3D` (`self.ball1`) (`KismetMathLibrary.Conv_DoubleToVector` _output_get)))

(fn `UserConstructionScript`)